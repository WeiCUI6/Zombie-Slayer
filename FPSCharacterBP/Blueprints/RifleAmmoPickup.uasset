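; Rifle ammo pickup actor that grants extra ammo when a ThirdPersonCharacter overlaps it.
; On overlap it adds one ClipSize to the MaxAmmo of the character's EquippedWeapon, with no check on weapon type.
; It then destroys itself and spawns an explosion particle effect and a quieter explosion sound at its location.
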(event EventBeginPlay)

(event Collision|EventActorBeginOverlap
  (params (OtherActor :type Actor%20Object%20Reference))
  (bind _asthird_person_character (Utilities|Casting|CastToThirdPersonCharacter OtherActor))
  (Variables|/Game/ThirdPersonBP/Blueprints/Weapons/AK47/Weapon_Base.Weapon_Base_C|SetMaxAmmo (Variables|/Game/ThirdPersonBP/Blueprints/ThirdPersonCharacter.ThirdPersonCharacter_C|GetEquippedWeapon _asthird_person_character) (+ (Variables|/Game/ThirdPersonBP/Blueprints/Weapons/AK47/Weapon_Base.Weapon_Base_C|GetMaxAmmo (Variables|/Game/ThirdPersonBP/Blueprints/ThirdPersonCharacter.ThirdPersonCharacter_C|GetEquippedWeapon _asthird_person_character)) (Variables|/Game/ThirdPersonBP/Blueprints/Weapons/AK47/Weapon_Base.Weapon_Base_C|GetClipSize (Variables|/Game/ThirdPersonBP/Blueprints/ThirdPersonCharacter.ThirdPersonCharacter_C|GetEquippedWeapon _asthird_person_character))))
  (Actor|DestroyActor)
  (Effects|SpawnEmitteratLocation "/Game/StarterContent/Particles/P_Explosion.P_Explosion" (Transformation|GetActorLocation))
  (Audio|SpawnSoundatLocation "/Game/StarterContent/Audio/Explosion_Cue.Explosion_Cue" (Transformation|GetActorLocation) "0, 0, 0" 0.3 1.0 0.0 0 0))

(event EventTick
  (params (DeltaSeconds :type Float%20%28single-precision%29)))

(fn ConstructionScript)