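; Thrown grenade actor that launches itself along the player's aim and explodes on a short timer.
; On BeginPlay it applies an impulse to its physics mesh along player 0's control rotation.
; After a delay it spawns an attached explosion emitter and sound, then destroys every SimpleAI overlapping its sphere, with no damage calculation.
; The grenade destroys itself a few seconds later.
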(event EventBeginPlay
  (bind _staticmesh (Variables|Default|GetStaticMesh))
  (Physics|AddImpulse (Variables|Default|GetStaticMesh) (* (Math|Rotator|GetRotationXVector (Pawn|GetControlRotation (Game|GetPlayerController 0) :!class /Script/Engine.Controller)) "1200.000000,1200.000000,1200.000000") "None" false)
  (Utilities|FlowControl|Delay 1.0)
  (Effects|SpawnEmitterAttached "/Game/StarterContent/Particles/P_Explosion.P_Explosion" _staticmesh "None" "0, 0, 0" "0, 0, 0" "45.000000,45.000000,45.000000")
  (Audio|SpawnSoundatLocation "/Game/StarterContent/Audio/Explosion_Cue.Explosion_Cue" (Transformation|GetWorldLocation _staticmesh) "0, 0, 0" 1.0 1.0 0.0 0 0)
  (Actor|DestroyActor (Collision|GetOverlappingActors (Variables|Default|GetSphere) "/Game/ThirdPersonBP/Blueprints/SimpleAI.SimpleAI_C" :!class /Script/Engine.PrimitiveComponent))
  (Utilities|FlowControl|Delay 5.0)
  (Actor|DestroyActor))

(event Collision|EventActorBeginOverlap
  (params (OtherActor :type Actor%20Object%20Reference)))

(event EventTick
  (params (DeltaSeconds :type Float%20%28single-precision%29)))

(fn ConstructionScript)